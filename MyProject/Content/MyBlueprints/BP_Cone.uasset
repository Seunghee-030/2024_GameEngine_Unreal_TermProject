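; BP_Cone is a goal pickup that disappears when anything overlaps its Capsule and scores when that actor is BP_Banana.
; On overlap it prints the actor's name and destroys itself before casting, then increments the GoalCount stored on the banana.
; It is meant to copy the count to PlayerUI and print it, but that cast has no object wired in, so those steps never run.
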(event OnComponentBeginOverlap(Capsule)
  (params (OverlappedComponent :type Primitive%20Component%20Object%20Reference) (OtherActor :type Actor%20Object%20Reference) (OtherComp :type Primitive%20Component%20Object%20Reference) (OtherBodyIndex :type Integer) (bFromSweep :type Boolean) (SweepResult :type Hit%20Result%20Structure%20%28by%20ref%29))
  (Development|PrintString (Utilities|GetDisplayName OtherActor))
  (Actor|DestroyActor)
  (bind _asbp_banana (Utilities|Casting|CastToBP_Banana OtherActor))
  (bind _output_get (Variables|/Game/MyBlueprints/BP_Banana.BP_Banana_C|SetGoalCount _asbp_banana (+ (Variables|/Game/MyBlueprints/BP_Banana.BP_Banana_C|GetGoalCount _asbp_banana) 1)))
  (bind _asplayer_ui (Utilities|Casting|CastToPlayerUI))
  (Variables|/Game/MyBlueprints/PlayerUI.PlayerUI_C|SetGoal%20Count _asplayer_ui _output_get)
  (Development|PrintString (Utilities|String|ToString(Integer) _output_get))
  (Development|PrintString "Goal Count : "))

(event EventBeginPlay)

(event Collision|EventActorBeginOverlap
  (params (OtherActor :type Actor%20Object%20Reference)))

(event EventTick
  (params (DeltaSeconds :type Float%20%28single-precision%29)))

(fn ConstructionScript)